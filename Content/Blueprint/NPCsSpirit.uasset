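; NPC spirit that follows the player's SpiritCharacter and holds a one-time conversation on contact.
; Overlapping ChasingRange starts an AI MoveToActor toward the player, reissued every Tick while they stay in range.
; SphereCollision fires once if the NPC is interactable, calling NPCInteract with Replay and showing Conversation text in a widget for five seconds.
; The construction script sets the Name text from CharName.
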(event OnComponentBeginOverlap(SphereCollision)
  (params (OverlappedComponent :type Primitive%20Component%20Object%20Reference) (OtherActor :type Actor%20Object%20Reference) (OtherComp :type Primitive%20Component%20Object%20Reference) (OtherBodyIndex :type Integer) (bFromSweep :type Boolean) (SweepResult :type Hit%20Result%20Structure%20%28by%20ref%29))
  (if (not (Variables|Default|GetbIsPlayerInteracted?))
    (if (Variables|Default|GetbIsInteractable?)
      (bind _asspirit_character (Utilities|Casting|CastToSpiritCharacter OtherActor))
      (Variables|Default|SetbIsPlayerInteracted? true)
      (Rendering|SetVisibility (Variables|Default|GetConversationWidget) true false)
      (Default|NPCInteract _asspirit_character (Variables|Default|GetReplay))
      (CallFunction|SetText)
      (Utilities|FlowControl|Delay 5.0)
      (Rendering|SetVisibility (Variables|Default|GetConversationWidget) false false))))

(event OnComponentBeginOverlap(ChasingRange)
  (params (OverlappedComponent :type Primitive%20Component%20Object%20Reference) (OtherActor :type Actor%20Object%20Reference) (OtherComp :type Primitive%20Component%20Object%20Reference) (OtherBodyIndex :type Integer) (bFromSweep :type Boolean) (SweepResult :type Hit%20Result%20Structure%20%28by%20ref%29))
  (bind _asspirit_character (Utilities|Casting|CastToSpiritCharacter OtherActor))
  (AI|Navigation|MovetoActor (AI|GetAIController self) _asspirit_character 1.2e+02 true true true 0))

(event EventTick
  (params (DeltaSeconds :type Float%20%28single-precision%29))
  (bind _chasingrange (Variables|Default|GetChasingRange))
  (bind _overlappingactors (Collision|GetOverlappingActors _chasingrange 0 :!class /Script/Engine.PrimitiveComponent))
  (if (> (Utilities|Array|Length _overlappingactors) 0)
    (for _array_element _overlappingactors
      (bind _asspirit_character (Utilities|Casting|CastToSpiritCharacter _array_element))
      (AI|Navigation|MovetoActor (AI|GetAIController self) _asspirit_character 1e+02 true true true 0))))

(fn ConstructionScript
  (Rendering|Components|TextRender|SetText (Variables|Default|GetName) (Variables|Default|GetCharName)))

(fn SetText
  (Rendering|Components|TextRender|SetText (Variables|/Game/Blueprint/Widgets/ConversationWidget.ConversationWidget_C|GetConversationTxt (.AsConversation%20Widget (Utilities|Casting|CastToConversationWidget (UserInterface|GetWidget (Variables|Default|GetConversationWidget))))) (Variables|Default|GetConversation)))
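; NPC actor that shows a name label and delivers a one-time line of dialogue when the main character approaches.
; The construction script writes CharName to the Name label.
; On the first sphere overlap by MainCharacter while IsInteractable, it shows the conversation widget, passes Replay to the character's NPCInteract, fills in the Conversation text, and hides the widget after a short delay.
; IsPlayerInteracted is never reset here, so the exchange does not repeat.
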(event OnComponentBeginOverlap(SphereCollision)
  (params (OverlappedComponent :type Primitive%20Component%20Object%20Reference) (OtherActor :type Actor%20Object%20Reference) (OtherComp :type Primitive%20Component%20Object%20Reference) (OtherBodyIndex :type Integer) (bFromSweep :type Boolean) (SweepResult :type Hit%20Result%20Structure%20%28by%20ref%29))
  (if (Variables|Default|GetbIsInteractable?)
    (if (not (Variables|Default|GetbIsPlayerInteracted?))
      (bind _asmain_character (Utilities|Casting|CastToMainCharacter OtherActor))
      (Variables|Default|SetbIsPlayerInteracted? true)
      (Rendering|SetVisibility (Variables|Default|GetConversationWidget) true false)
      (Default|NPCInteract _asmain_character (Variables|Default|GetReplay))
      (CallFunction|SetText)
      (Utilities|FlowControl|Delay 5.0)
      (Rendering|SetVisibility (Variables|Default|GetConversationWidget) false false))))

(event OnComponentEndOverlap(SphereCollision)
  (params (OverlappedComponent :type Primitive%20Component%20Object%20Reference) (OtherActor :type Actor%20Object%20Reference) (OtherComp :type Primitive%20Component%20Object%20Reference) (OtherBodyIndex :type Integer)))

(event EventBeginPlay)

(event Collision|EventActorBeginOverlap
  (params (OtherActor :type Actor%20Object%20Reference)))

(event EventTick
  (params (DeltaSeconds :type Float%20%28single-precision%29)))

(fn ConstructionScript
  (Rendering|Components|TextRender|SetText (Variables|Default|GetName) (Variables|Default|GetCharName)))

(fn SetText
  (Rendering|Components|TextRender|SetText (Variables|/Game/Blueprint/Widgets/ConversationWidget.ConversationWidget_C|GetConversationTxt (.AsConversation%20Widget (Utilities|Casting|CastToConversationWidget (UserInterface|GetWidget (Variables|Default|GetConversationWidget))))) (Variables|Default|GetConversation)))